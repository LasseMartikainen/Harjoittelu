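; Player-controlled cue ball for a billiards game, with a following camera and a stick.
; At start, a physics handle drags the ball by mouse until left-click release, after which Tick removes the start-area constraint and indicator.
; Mouse X then aims ball, camera and debug trace; holding Stroke charges force and draws the stick back, releasing applies an impulse.
; Hand-ball reset after potting and angle wrapping are unwired, marked not working.
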(event EventBeginPlay
  (bind _sm_ball (Variables|Default|GetSM_Ball))
  ;[1 1 1] SetUp
  (Variables|Default|SetStartMode true)
  (Physics|SetSimulatePhysics (Variables|Default|GetSM_Ball) true)
  ;[1 1 1] Handball movement
  (Class|PhysicsHandleComponent|GrabComponentatLocation (Variables|Default|GetPhysicsHandle) _sm_ball "None" (Transformation|GetWorldLocation _sm_ball)))

(event Collision|EventActorBeginOverlap
  (params (OtherActor :type Actor%20Object%20Reference))
  ;[1 1 1] Hand ball set up (not working)
)

(event EventTick
  (params (DeltaSeconds :type Float%20%28single-precision%29))
  (bind _returnvalue (Game|GetPlayerController 0))
  (bind _sm_ball (Variables|Default|GetSM_Ball))
  (bind _sm_ball_2 (Variables|Default|GetSM_Ball))
  (bind _sm_ball_3 (Variables|Default|GetSM_Ball))
  (bind _startareaconstraint (Variables|Default|GetStartAreaConstraint))
  (bind _returnvalue_2 (Transformation|GetWorldLocation _sm_ball_3))
  (bind _returnvalue_3 (Transformation|GetWorldLocation _sm_ball))
  (bind (_worldlocation _worlddirection) (Game|Player|ConvertMouseLocationToWorldSpace _returnvalue))
  (bind (_x _y) (Class|KismetMathLibrary|BreakVector3f _returnvalue_3))
  (bind (_x_2 _y_2) (Class|KismetMathLibrary|BreakVector3f _returnvalue_2))
  ;[1 1 1] Handball movement
  (Physics|Components|PhysicsHandle|SetTargetLocation (Variables|Default|GetPhysicsHandle) (+ _worldlocation (* _worlddirection (* (Math|Vector|VectorLength (Math|Vector|GetUnitDirection(Vector) _worlddirection _returnvalue_2)) 2.5e+02))))
  ;[1 1 1] End of SetUp
  (if (Variables|Default|GetStartMode)
    _
    (elif (Utilities|IsValid _startareaconstraint)
      (Components|DestroyComponent _startareaconstraint)
      (bind _outactors (Actor|GetAllActorswithTag "StartAreaIndicator"))
      (Actor|DestroyActor _outactors)))
  ;[1 1 1] Camera movement
  (bind _output_get (Variables|Default|SetNewCameraLocation (Math|Vector|MakeVector (+ _x_2 (* (Math|Trig|Cos(Degrees) (Variables|Default|GetHitDirection)) -5e+01)) (+ _y_2 (* (Math|Trig|Sin(Degrees) (Variables|Default|GetHitDirection)) -5e+01)) (Variables|Default|GetCameraHeight))))
  ;[1 1 1] Cue ball rotation
  (Transformation|SetWorldRotation (Variables|Default|GetSM_Ball) (Math|Rotator|MakeRotator 0.0 0.0 (Variables|Default|GetHitDirection)) false false)
  ;[1 1 1] Line trace
  (bind _output_get_2 (Variables|Default|SetTraceStartLocation (Math|Vector|MakeVector _x _y 8e+01)))
  (bind _outhit_distance (|Trace _output_get_2 (+ _output_get_2 (* (Math|Vector|GetForwardVector (Transformation|GetWorldRotation _sm_ball)) (Variables|Default|GetTraceDistance)))))
  (Development|PrintString (Utilities|String|ToString(Float) _outhit_distance) true true "(R=0.000000,G=0.660000,B=1.000000,A=1.000000)" 0.1)
  (Transformation|SetWorldLocationAndRotation (Variables|Default|GetCamera) _output_get (Math|Rotator|MakeRotator 0.0 3e+02 (Variables|Default|GetHitDirection)) false false)
  ;[1 1 1] Rotate when it is not handball
  (if (Variables|Default|GetHandMode)
    ;[1 1 1] HandBall
    (Class|PhysicsHandleComponent|GrabComponentatLocation (Variables|Default|GetPhysicsHandle) _sm_ball_2 "None" (Transformation|GetWorldLocation _sm_ball_2))
    (Collision|SetCollisionEnabled _sm_ball_2 "NoCollision")
    (elif (not (Variables|Default|GetStartMode))
      (bind _output_get_3 (Variables|Default|SetHitDirection (/ (.LocationX (Class|WidgetLayoutLibrary|GetMousePositionScaledbyDPI (Game|GetPlayerController 0))) 2.0))))))

(event Input|ActionEvents|InputActionStroke
  (params (Key :type Key%20Structure :default "None"))
  (bind _maximumforce (Variables|Default|GetMaximumForce))
  (bind _bp_stick (Variables|Default|GetBP_Stick))
  (bind _bp_stick_2 (Variables|Default|GetBP_Stick))
  (bind _hitdirection (Variables|Default|GetHitDirection))
  ;[1 1 1] Hitting the cue ball
  (:Pressed
    (bind _output_get (Variables|Default|SetSpacePressed true))
    ;[1 1 1] Stick movement
    (Rendering|SetVisibility _bp_stick true false)
    (bind _output_get_2 (Variables|Default|SetStick%20location (Variables|/Script/Engine.SceneComponent|GetRelativeLocation _bp_stick)))
    (if _output_get :!label _label
      (bind _output_get_3 (Variables|Default|SetHitForce (+ 33.3 (Variables|Default|GetHitForce))))
      (if (>= _output_get_3 _maximumforce)
        (Variables|Default|SetHitForce _maximumforce)
        (else
          (Transformation|AddLocalOffset _bp_stick (Math|Vector|MakeVector (* (Variables|Default|GetHitForce) -0.001) 0.0 (* (Variables|Default|GetHitForce) -0.02)) false false)
          (Variables|Default|SetOffsetVector (Math|Vector|MakeVector (+ (* (Variables|Default|GetHitForce) -0.001) (.X (Class|KismetMathLibrary|BreakVector3f (Variables|Default|GetOffsetVector)))) (.Y (Class|KismetMathLibrary|BreakVector3f (Variables|Default|GetOffsetVector))) (+ (* (Variables|Default|GetHitForce) -0.02) (.Z (Class|KismetMathLibrary|BreakVector3f (Variables|Default|GetOffsetVector))))))))
      (Development|PrintString (Utilities|String|ToString(Float) _output_get_3))
      (Utilities|FlowControl|Delay 0.5)
      (goto _label)))
  (:Released
    (Variables|Default|SetSpacePressed false)
    (if (Actor|ActorHasTag "CueBall")
      (bind _output_get_4 (Variables|Default|SetImpulseDirection (Math|Vector|MakeVector (* (Math|Trig|Cos(Degrees) _hitdirection) (Variables|Default|GetHitForce)) (* (Math|Trig|Sin(Degrees) _hitdirection) (Variables|Default|GetHitForce)) 0.0)))
      (Physics|AddImpulse (Variables|Default|GetSM_Ball) _output_get_4 "None" false)
      (Variables|Default|SetHitForce 0.0)
      (Transformation|AddLocalOffset _bp_stick_2 (* (Variables|Default|GetOffsetVector) "-1.000000,-1.000000,-1.000000") false false)
      (Audio|PlaySoundatLocation "/Game/BilliardsAssets/BallHit.BallHit" _output_get_2 "0, 0, 0" 1.0 1.0 0.0 0 0 0 0)
      (Utilities|FlowControl|Delay 0.1)
      ;;[1 1 1] Reset stick location
      (Rendering|SetVisibility _bp_stick_2 false false)
      (Transformation|SetRelativeLocation (Variables|Default|GetBP_Stick) (Variables|Default|GetStick%20location) false true))))

(event Input|MouseEvents|LeftMouseButton
  (params (Key :type Key%20Structure :default "None"))
  ;[1 1 1] Drop handball
  (:Released
    (Physics|Components|PhysicsHandle|ReleaseComponent (Variables|Default|GetPhysicsHandle))
    (Variables|Default|SetHandMode false)
    (Variables|Default|SetStartMode false)
    (Collision|SetCollisionEnabled (Variables|Default|GetSM_Ball) "QueryAndPhysics")))

(fn ConstructionScript)