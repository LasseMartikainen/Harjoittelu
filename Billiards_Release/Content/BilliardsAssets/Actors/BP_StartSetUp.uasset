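; BP_StartSetUp sets up the billiards table at BeginPlay, starting background music and racking the balls in the start triangle.
; It spawns a BP_Ball at each TargetPoint in the level, pairing them by index with the numbers from StartLocations, which the comments describe as randomized.
; Each ball receives its number through SetBallNumber, which also selects its mesh material from BallMaterials.
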(event EventBeginPlay
  (AddComponent|AddAudioComponent false) ; Backround music
  ;[1 1 1] Start triangle
  (bind _outactors (Actor|GetAllActorsOfClass "/Script/Engine.TargetPoint")) ; Get ball locations in game
  (for (_array_element _array_index) (Class|StartSetUp|StartLocations)
    (bind _returnvalue (Game|SpawnActorfromClass "/Game/BilliardsAssets/Actors/BP_Ball.BP_Ball_C" (Transformation|GetActorTransform (Utilities|Array|Get(acopy) _outactors _array_index)) "Undefined" "MultiplyWithRoot" 0 0))
    (Rendering|Material|SetMaterial (Actor|GetComponentbyClass _returnvalue "/Script/Engine.StaticMeshComponent") 0 (Utilities|Array|Get(acopy) (Class|StartSetUp|BallMaterials) (- (Class|BasicBall|SetBallNumber _returnvalue _array_element) 1)))))

(fn ConstructionScript)