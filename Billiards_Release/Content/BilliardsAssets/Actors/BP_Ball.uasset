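; BP_Ball is a billiards ball actor that handles being potted.
; On overlap, it finds components tagged "Pot" on the other actor and reads the pot number from each component's second tag.
; It passes its ball number and that pot number to the first top-level BP_ScoreWidget's Potting function, then destroys itself.
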(event Collision|EventActorBeginOverlap
  (params (OtherActor :type Actor%20Object%20Reference))
  ;[1 1 1] The act of potting
  (for _array_element (Actor|GetComponentsbyTag OtherActor "/Script/Engine.ActorComponent" "Pot")
    (bind _foundwidgets (Widget|GetAllWidgetsOfClass "/Game/UI/BP_ScoreWidget.BP_ScoreWidget_C" true))
    (Class|ScoreWidget|Potting (Utilities|Array|Get(acopy) _foundwidgets) (Class|BasicBall|GetBallNumber) (Math|Conversions|ToInteger(Byte) (Utilities|String|ToString(Name) (Utilities|Array|Get(acopy) (Variables|/Script/Engine.ActorComponent|GetComponentTags _array_element) 1))))
    (Actor|DestroyActor)))

(fn ConstructionScript)